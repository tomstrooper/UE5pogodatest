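; BP_QuestMapPro_HiddenObject is a QuestMap world actor that represents a hidden object as an overlap sphere with a billboard.
; The construction script sizes OverlapTrigger from ObjectRadius, then calls SetState to raise MaterialBillboard to BillboardHeight for editor visibility.
; GetActorReference returns the actor itself; this file contains no overlap or discovery logic.
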(fn ConstructionScript
  (Components|Sphere|SetSphereRadius (Variables|Default|GetOverlapTrigger) (Variables|Configuration|GetObjectRadius) true) ; Update OverlapTrigger to represent the\nsize of the object based on Object Radius.
  (CallFunction|SetState))

(fn SetState
  (Transformation|SetRelativeLocation (Variables|Default|GetMaterialBillboard) (Math|Vector|MakeVector 0.0 0.0 (Variables|Configuration|GetBillboardHeight)) false false) ; Set billboard height for better editor visibility.
  (return))

(fn GetActorReference
  (return self))