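; Point-of-interest actor for the QuestMap system that shows an icon billboard in the world.
; SetState runs on construction and BeginPlay, raising the billboard to BillboardHeight and creating a dynamic instance of the billboard material if none exists.
; It then applies the Icon texture and Color to that instance.
; GetActorReference returns the actor itself.
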(event EventBeginPlay
  (Configuration|SetState))

(fn ConstructionScript
  (Configuration|SetState) ; Set POI state.
)

(fn SetState
  (Transformation|SetRelativeLocation (Variables|Default|GetMaterialBillboard) (Math|Vector|MakeVector 0.0 0.0 (Variables|Configuration|GetBillboardHeight)) false false)
  (Variables|Default|GetBillboardMat
    (:then
      _)
    (:else
      (bind _returnvalue (Rendering|Material|CreateDynamicMaterialInstance "/Game/QuestMap/Materials/Other/BaseMaterials/M_QuestMapPro_BillboardMaterial.M_QuestMapPro_BillboardMaterial" "None" "None" :!class /Script/Engine.KismetMaterialLibrary))
      (bind _output_get (Variables|Default|SetBillboardMat _returnvalue))
      (Rendering|Material|SetMaterial (Variables|Default|GetMaterialBillboard) 0 _output_get)))
  (Rendering|Material|SetTextureParameterValue (Variables|Default|GetBillboardMat) "Texture" (Variables|Configuration|GetIcon))
  (Rendering|Material|SetVectorParameterValue (Variables|Default|GetBillboardMat) "Color" (Variables|Configuration|GetColor) :!class /Script/Engine.MaterialInstanceDynamic)
  (return))

(fn GetActorReference
  (return self))