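; BP_QuestMapPro_Quest is a world actor marking a quest as a Location, Area or Attached type.
; The construction script configures the trigger sphere by type and radius, scaling and tinting a decal for Area quests.
; Other types destroy the decal, and Attached quests also snap to their target actor.
; UpdateMaterial recolors the beacon cylinder through a lazily created, cached dynamic material instance.
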(event Custom|UpdateMaterial
  (params (Value :type Linear%20Color%20Structure))
  (Variables|Default|GetBeaconMat
    (:then
      _)
    (:else
      (bind _returnvalue (Rendering|Material|CreateDynamicMaterialInstance (Variables|Default|GetCylinder) 0 "/Game/QuestMap/Materials/Other/MI_QuestMapPro_WaypointRay.MI_QuestMapPro_WaypointRay" "None" :!class /Script/Engine.PrimitiveComponent))
      (Variables|Default|SetBeaconMat _returnvalue)))
  (Rendering|Material|SetVectorParameterValue (Variables|Default|GetBeaconMat) "Color" Value :!class /Script/Engine.MaterialInstanceDynamic))

(fn ConstructionScript
  (bind _arearadius (Variables|Default|GetAreaRadius))
  (bind _returnvalue (/ _arearadius 1e+03))
  (Collision|SetCollisionEnabled (Variables|Default|GetQuestArea) (Utilities|Select :Index (Variables|Default|GetQuestClass) :NewEnumerator0 "NoCollision" :NewEnumerator1 "QueryOnly" :NewEnumerator2 "NoCollision")) ; Set collision to query for quest areas, and\nnone for all other types.
  (Components|Sphere|SetSphereRadius (Variables|Default|GetQuestArea) (Variables|Default|GetAreaRadius) true) ; Set the collider radius.
  (switch Utilities|FlowControl|Switch|SwitchonE_QuestMapPro_QuestClass (Variables|Default|GetQuestClass)
    (:NewEnumerator0
      (Components|DestroyComponent (Variables|Default|GetQuestAreaDecal)) ; Quest area decal not needed for location quests, so destroy it.
    )
    (:NewEnumerator1
      (Transformation|SetWorldScale3D (Variables|Default|GetQuestAreaDecal) (Math|Vector|MakeVector _returnvalue _returnvalue _returnvalue)) ; Scale the decal to fit the quest area\nentirely.
      (bind _returnvalue_2 (Rendering|Material|CreateDynamicMaterialInstance (Variables|Default|GetQuestAreaDecal) :!class /Script/Engine.DecalComponent)) ; Create a dynamic instance of decal material.
      (Rendering|Material|SetVectorParameterValue _returnvalue_2 "Color" (Variables|Default|GetQuestColor) :!class /Script/Engine.MaterialInstanceDynamic) ; Update decal color.
    )
    (:NewEnumerator2
      (Transformation|AttachActorToActor self (Variables|Default|GetActorToAttachTo) "None" "SnapToTarget" "SnapToTarget" "SnapToTarget" true) ; Attach quest actor to the appropriate actor.
      (Components|DestroyComponent (Variables|Default|GetQuestAreaDecal)) ; Quest area decal not needed for attached quests, so destroy it.
    )))