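; A quest map landmark world actor that shows an icon billboard and carries an overlap trigger for a discoverable location.
; SetState runs on construction and BeginPlay, setting billboard height, dynamic material icon and color, and enabling either a sphere or box trigger while zeroing the other.
; Accessors expose the actor, discoverable type, landmark state and navigation point.
; UpdateLandmarkState only stores the state; visuals always use DiscoveredColor, and no overlap handling lives here.
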(event EventBeginPlay
  (Configuration|SetState))

(fn ConstructionScript
  (Configuration|SetState))

(fn SetState
  (Transformation|SetRelativeLocation (Variables|Default|GetMaterialBillboard) (Math|Vector|MakeVector 0.0 0.0 (Variables|Configuration|GetBillboardHeight)) false true) ; Set billboard height per location.
  (Variables|OperatingValues|GetBillboardMat
    (:then
      _)
    (:else
      (bind _returnvalue (Rendering|Material|CreateDynamicMaterialInstance "/Game/QuestMap/Materials/Other/BaseMaterials/M_QuestMapPro_BillboardMaterial.M_QuestMapPro_BillboardMaterial" "None" "None" :!class /Script/Engine.KismetMaterialLibrary))
      (bind _output_get (Variables|OperatingValues|SetBillboardMat _returnvalue))
      (Rendering|Material|SetMaterial (Variables|Default|GetMaterialBillboard) 0 _output_get)))
  (Rendering|Material|SetTextureParameterValue (Variables|OperatingValues|GetBillboardMat) "Texture" (Variables|Configuration|GetLandmarkIcon))
  (Rendering|Material|SetVectorParameterValue (Variables|OperatingValues|GetBillboardMat) "Color" (Variables|Configuration|GetDiscoveredColor) :!class /Script/Engine.MaterialInstanceDynamic)
  (Collision|SetCollisionEnabled (Variables|Default|GetOverlapTriggerSphere) (select (Variables|Configuration|GetUseBoxCollision) "NoCollision" "QueryOnly")) ; Set sphere collision based on UseBoxCollision appropriately.
  (Collision|SetCollisionEnabled (Variables|Default|GetOverlapTriggerBox) (select (Variables|Configuration|GetUseBoxCollision) "QueryOnly" "NoCollision")) ; Set box collision based on UseBoxCollision appropriately.
  (Components|Sphere|SetSphereRadius (Variables|Default|GetOverlapTriggerSphere) (Math|Float|SelectFloat 0.0 (Variables|Configuration|GetColliderRadius) (Variables|Configuration|GetUseBoxCollision)) true) ; Set sphere radius based on ColliderRadius, taking into\naccount UseBoxCollision appropriately.
  (Components|Box|SetBoxExtent (Variables|Default|GetOverlapTriggerBox) (Math|Vector|SelectVector (Variables|Configuration|GetColliderExtent) "0, 0, 0" (Variables|Configuration|GetUseBoxCollision)) true) ; Set box extent based on ColliderExtent, taking into\naccount UseBoxCollision appropriately.
  (return))

(fn UpdateLandmarkState
  (params (NewState :type E_QuestMapPro_LandmarkState%20Enum :default "NewEnumerator0"))
  (Variables|OperatingValues|SetState NewState)
  (return))

(fn GetActorReference
  (return self))

(fn GetDiscoverableObject
  (return self "NewEnumerator0"))

(fn GetLandmarkState
  (return (Variables|OperatingValues|GetState)))

(fn GetNavPoint
  (return (Variables|Configuration|GetNavigationPoint)))