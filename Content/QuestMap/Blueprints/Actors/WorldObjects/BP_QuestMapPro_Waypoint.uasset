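; Waypoint world actor for the QuestMap system, with a colored ray beacon on a cylinder mesh and an optional indicator component.
; UpdateMaterial lazily creates a dynamic instance of the waypoint ray material and sets its Color parameter.
; UpdateIndicator toggles indicator visibility in game, and the construction script unhides it when UseIndicator is set.
; GetActorReference and GetDiscoverableObject expose the actor itself, the latter paired with a discoverable type.
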(event Custom|UpdateMaterial
  (params (Value :type Linear%20Color%20Structure))
  (Variables|Default|GetBeaconMat
    (:then
      _)
    (:else
      (bind _returnvalue (Rendering|Material|CreateDynamicMaterialInstance (Variables|Default|GetCylinder) 0 "/Game/QuestMap/Materials/Other/MI_QuestMapPro_WaypointRay.MI_QuestMapPro_WaypointRay" "None" :!class /Script/Engine.PrimitiveComponent))
      (Variables|Default|SetBeaconMat _returnvalue)))
  (Rendering|Material|SetVectorParameterValue (Variables|Default|GetBeaconMat) "Color" Value :!class /Script/Engine.MaterialInstanceDynamic))

(event Custom|UpdateIndicator
  (params (Enabled? :type Boolean))
  (Variables|Default|SetUseIndicator Enabled?)
  (Development|SetHiddeninGame (Variables|Default|GetIndicator) (not (Variables|Default|GetUseIndicator)) false))

(fn ConstructionScript
  (if (Variables|Default|GetUseIndicator)
    (Development|SetHiddeninGame (Variables|Default|GetIndicator) false false)))

(fn GetActorReference
  (return self))

(fn GetDiscoverableObject
  (return self "NewEnumerator2"))