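; Helper actor for the Quest Map Pro character that detects nearby map objects and reports them to the QuestMapManager.
; Separate trigger volumes catch discoverables, landmarks, POIs, hidden objects, NPCs or players, and quest or landmark areas, filtering by class or interface.
; Construction applies manager-configured sizes, Z offset and debug visibility, and destroys manually placed copies.
; Discovery overlaps are enabled after a short BeginPlay delay, once initialized.
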(event OnComponentBeginOverlap(LandmarkTrigger)
  (params (OverlappedComponent :type Primitive%20Component%20Object%20Reference) (OtherActor :type Actor%20Object%20Reference) (OtherComp :type Primitive%20Component%20Object%20Reference) (OtherBodyIndex :type Integer) (bFromSweep :type Boolean) (SweepResult :type Hit%20Result%20Structure%20%28by%20ref%29))
  ;[1 1 1] Landmark Trigger Overlap.
  (if (== (Utilities|GetClass OtherActor) "/Game/QuestMap/Blueprints/Actors/WorldObjects/BP_QuestMapPro_Landmark.BP_QuestMapPro_Landmark_C") ; Ensure the overlapping actor is a landmark actor.
    (bind _questmapmanager (Variables|Default|GetQuestMapManager)
      (:then
        (bind _landmark (Class|BPIntQuestMapProLandmarkActor|GetActorReference(Message) OtherActor))
        (Default|ProcessLandmark _questmapmanager true _landmark) ; Activate a new overlap event.
      )
      (:else))))

(event OnComponentEndOverlap(LandmarkTrigger)
  (params (OverlappedComponent :type Primitive%20Component%20Object%20Reference) (OtherActor :type Actor%20Object%20Reference) (OtherComp :type Primitive%20Component%20Object%20Reference) (OtherBodyIndex :type Integer))
  ;[1 1 1] Landmark Trigger Overlap.
  (if (== (Utilities|GetClass OtherActor) "/Game/QuestMap/Blueprints/Actors/WorldObjects/BP_QuestMapPro_Landmark.BP_QuestMapPro_Landmark_C") ; Ensure the overlapping actor is a landmark actor.
    (bind _questmapmanager (Variables|Default|GetQuestMapManager)
      (:then
        (bind _landmark (Class|BPIntQuestMapProLandmarkActor|GetActorReference(Message) OtherActor))
        (Default|ProcessLandmark _questmapmanager false _landmark) ; Activate an end overlap event.
      )
      (:else))))

(event OnComponentEndOverlap(CapsuleTrigger)
  (params (OverlappedComponent :type Primitive%20Component%20Object%20Reference) (OtherActor :type Actor%20Object%20Reference) (OtherComp :type Primitive%20Component%20Object%20Reference) (OtherBodyIndex :type Integer))
  (bind _returnvalue (Utilities|GetClass OtherActor))
  ;[1 1 1] CapsuleOverlap
  (if (== _returnvalue "/Game/QuestMap/Blueprints/Actors/WorldObjects/BP_QuestMapPro_Quest.BP_QuestMapPro_Quest_C") ; Ensure the overlapping actor is the correct class for quest area overlaps.
    (bind _questmapmanager (Variables|Default|GetQuestMapManager)
      (:then
        (Default|ProcessQuestArea _questmapmanager false) ; Activate an end overlap event.
      )
      (:else))
    (elif (== _returnvalue "/Game/QuestMap/Blueprints/Actors/WorldObjects/BP_QuestMapPro_Landmark.BP_QuestMapPro_Landmark_C") ; Is the overlapping actor a landmark?
      (bind _questmapmanager_2 (Variables|Default|GetQuestMapManager)
        (:then
          (bind _landmark (Class|BPIntQuestMapProLandmarkActor|GetActorReference(Message) OtherActor))
          (Default|OverlapLandmarkArea _questmapmanager_2 false _landmark) ; Activate an end overlap event.
        )
        (:else)))))

(event OnComponentBeginOverlap(POITrigger)
  (params (OverlappedComponent :type Primitive%20Component%20Object%20Reference) (OtherActor :type Actor%20Object%20Reference) (OtherComp :type Primitive%20Component%20Object%20Reference) (OtherBodyIndex :type Integer) (bFromSweep :type Boolean) (SweepResult :type Hit%20Result%20Structure%20%28by%20ref%29))
  ;[1 1 1] Point of Interest Trigger Overlap.
  (if (== (Utilities|GetClass OtherActor) "/Game/QuestMap/Blueprints/Actors/WorldObjects/BP_QuestMapPro_POI.BP_QuestMapPro_POI_C") ; Ensure the overlapping actor is a POI actor.
    (bind _questmapmanager (Variables|Default|GetQuestMapManager)
      (:then
        (bind _poi (Class|BPIntQuestMapProPOIActor|GetActorReference(Message) OtherActor))
        (Default|ProcessPOI _questmapmanager true _poi) ; Activate a new overlap event.
      )
      (:else))))

(event OnComponentEndOverlap(POITrigger)
  (params (OverlappedComponent :type Primitive%20Component%20Object%20Reference) (OtherActor :type Actor%20Object%20Reference) (OtherComp :type Primitive%20Component%20Object%20Reference) (OtherBodyIndex :type Integer))
  ;[1 1 1] Point of Interest Trigger Overlap.
  (if (== (Utilities|GetClass OtherActor) "/Game/QuestMap/Blueprints/Actors/WorldObjects/BP_QuestMapPro_POI.BP_QuestMapPro_POI_C") ; Ensure the overlapping actor is a POI actor.
    (bind _questmapmanager (Variables|Default|GetQuestMapManager)
      (:then
        (bind _poi (Class|BPIntQuestMapProPOIActor|GetActorReference(Message) OtherActor))
        (Default|ProcessPOI _questmapmanager false _poi) ; Activate an end overlap event.
      )
      (:else))))

(event OnComponentBeginOverlap(HiddenObjectTrigger)
  (params (OverlappedComponent :type Primitive%20Component%20Object%20Reference) (OtherActor :type Actor%20Object%20Reference) (OtherComp :type Primitive%20Component%20Object%20Reference) (OtherBodyIndex :type Integer) (bFromSweep :type Boolean) (SweepResult :type Hit%20Result%20Structure%20%28by%20ref%29))
  ;[1 1 1] Hidden Object Trigger Overlap.
  (if (== (Utilities|GetClass OtherActor) "/Game/QuestMap/Blueprints/Actors/WorldObjects/BP_QuestMapPro_HiddenObject.BP_QuestMapPro_HiddenObject_C") ; Ensure the overlapping actor is a hidden object actor.
    (bind _questmapmanager (Variables|Default|GetQuestMapManager)
      (:then
        (bind _object (Class|BPIntQuestMapProHiddenObjectActor|GetActorReference(Message) OtherActor))
        (Default|ProcessHiddenObject _questmapmanager true _object) ; Activate a new overlap event.
      )
      (:else))))

(event OnComponentEndOverlap(HiddenObjectTrigger)
  (params (OverlappedComponent :type Primitive%20Component%20Object%20Reference) (OtherActor :type Actor%20Object%20Reference) (OtherComp :type Primitive%20Component%20Object%20Reference) (OtherBodyIndex :type Integer))
  ;[1 1 1] Hidden Object Trigger Overlap.
  (if (== (Utilities|GetClass OtherActor) "/Game/QuestMap/Blueprints/Actors/WorldObjects/BP_QuestMapPro_HiddenObject.BP_QuestMapPro_HiddenObject_C") ; Ensure the overlapping actor is a hidden object actor.
    (bind _questmapmanager (Variables|Default|GetQuestMapManager)
      (:then
        (bind _object (Class|BPIntQuestMapProHiddenObjectActor|GetActorReference(Message) OtherActor))
        (Default|ProcessHiddenObject _questmapmanager false _object) ; Activate an end overlap event.
      )
      (:else))))

(event OnComponentBeginOverlap(NPCTrigger)
  (params (OverlappedComponent :type Primitive%20Component%20Object%20Reference) (OtherActor :type Actor%20Object%20Reference) (OtherComp :type Primitive%20Component%20Object%20Reference) (OtherBodyIndex :type Integer) (bFromSweep :type Boolean) (SweepResult :type Hit%20Result%20Structure%20%28by%20ref%29))
  (bind _returnvalue (Utilities|GetClass OtherActor))
  (bind _playerclass (Variables|Configuration|GetPlayerClass))
  ;[1 1 1] NPC Trigger Overlap.
  (if (Utilities|DoesObjectImplementInterface OtherActor "/Game/QuestMap/Blueprints/Interfaces/BPInt_QuestMapPro_NPCActor.BPInt_QuestMapPro_NPCActor_C") ; Ensure the overlapping actor has the interface required\nfor NPC actors.
    (bind _questmapmanager (Variables|Default|GetQuestMapManager)
      (:then
        (Default|ProcessNPC _questmapmanager true OtherActor) ; Activate a new overlap event.
      )
      (:else))
    (elif (or (Utilities|ClassIsChildOf _returnvalue _playerclass) (== _returnvalue _playerclass)) ; Check if the overlapping actor is the player\nclass, or a child thereof.
      (bind _questmapmanager_2 (Variables|Default|GetQuestMapManager)
        (:then
          (Default|ProcessPlayer _questmapmanager_2 true OtherActor) ; Activate a new overlap event.
        )
        (:else)))))

(event OnComponentEndOverlap(NPCTrigger)
  (params (OverlappedComponent :type Primitive%20Component%20Object%20Reference) (OtherActor :type Actor%20Object%20Reference) (OtherComp :type Primitive%20Component%20Object%20Reference) (OtherBodyIndex :type Integer))
  (bind _returnvalue (Utilities|GetClass OtherActor))
  (bind _playerclass (Variables|Configuration|GetPlayerClass))
  ;[1 1 1] NPC Trigger Overlap.
  (if (Utilities|DoesObjectImplementInterface OtherActor "/Game/QuestMap/Blueprints/Interfaces/BPInt_QuestMapPro_NPCActor.BPInt_QuestMapPro_NPCActor_C") ; Ensure the overlapping actor has the interface required\nfor NPC actors.
    (bind _questmapmanager (Variables|Default|GetQuestMapManager)
      (:then
        (Default|ProcessNPC _questmapmanager false OtherActor) ; Activate an end overlap event.
      )
      (:else))
    (elif (or (Utilities|ClassIsChildOf _returnvalue _playerclass) (== _returnvalue _playerclass)) ; Check if the overlapping actor is the player\nclass, or a child thereof.
      (bind _questmapmanager_2 (Variables|Default|GetQuestMapManager)
        (:then
          (Default|ProcessPlayer _questmapmanager_2 false OtherActor) ; Activate an end overlap event.
        )
        (:else)))))

(event OnComponentBeginOverlap(DiscoverTrigger)
  (params (OverlappedComponent :type Primitive%20Component%20Object%20Reference) (OtherActor :type Actor%20Object%20Reference) (OtherComp :type Primitive%20Component%20Object%20Reference) (OtherBodyIndex :type Integer) (bFromSweep :type Boolean) (SweepResult :type Hit%20Result%20Structure%20%28by%20ref%29))
  ;[1 1 1] Discover Trigger Overlap.
  (if (Utilities|DoesObjectImplementInterface OtherActor "/Game/QuestMap/Blueprints/Interfaces/BPInt_QuestMapPro_DiscoverableObject.BPInt_QuestMapPro_DiscoverableObject_C") ; Is the overlapping actor a discoverable object?
    (bind _questmapmanager (Variables|Default|GetQuestMapManager)
      (:then
        (Default|ProcessDiscovery _questmapmanager OtherActor) ; Process actor discovery.
      )
      (:else))))

(event OnComponentBeginOverlap(CapsuleTrigger)
  (params (OverlappedComponent :type Primitive%20Component%20Object%20Reference) (OtherActor :type Actor%20Object%20Reference) (OtherComp :type Primitive%20Component%20Object%20Reference) (OtherBodyIndex :type Integer) (bFromSweep :type Boolean) (SweepResult :type Hit%20Result%20Structure%20%28by%20ref%29))
  (bind _returnvalue (Utilities|GetClass OtherActor))
  ;[1 1 1] CapsuleOverlap
  (if (== _returnvalue "/Game/QuestMap/Blueprints/Actors/WorldObjects/BP_QuestMapPro_Quest.BP_QuestMapPro_Quest_C") ; Is this overlap event a quest area?
    (bind _questmapmanager (Variables|Default|GetQuestMapManager)
      (:then
        (Default|ProcessQuestArea _questmapmanager true) ; Activate a new overlap event.
      )
      (:else))
    (elif (== _returnvalue "/Game/QuestMap/Blueprints/Actors/WorldObjects/BP_QuestMapPro_Landmark.BP_QuestMapPro_Landmark_C") ; Is this overlap event a landmark?
      (bind _questmapmanager_2 (Variables|Default|GetQuestMapManager)
        (:then
          (bind _landmark (Class|BPIntQuestMapProLandmarkActor|GetActorReference(Message) OtherActor))
          (Default|OverlapLandmarkArea _questmapmanager_2 true _landmark) ; Activate a new overlap event.
        )
        (:else)))))

(event EventBeginPlay
  ;[1 1 1] Check if the character helper has initialized before allowing discoveries.
  (Utilities|FlowControl|Delay 0.2)
  (if (Variables|Configuration|GetInitialized)
    (Variables|/Script/Engine.PrimitiveComponent|SetbGenerateOverlapEvents (Variables|Default|GetDiscoverTrigger) true)))

(fn ConstructionScript
  (bind _capsuleradius (Variables|Configuration|GetCapsuleRadius))
  ;[1 1 1] Logic used to destroy actor if accidentally placed in world manually.
  (if (Variables|Configuration|GetAddedManually)
    (Actor|DestroyActor)
    (else
      (Transformation|AddRelativeLocation (Variables|Default|GetOffset) (Math|Vector|MakeVector 0.0 0.0 (Variables|Configuration|GetZOffset)) false true) ; Offset actor location on the character based on ZOffset\n(set in the Quest Map Manager component on the player\ncontroller).
      (Components|Sphere|SetSphereRadius (Variables|Default|GetLandmarkTrigger) (Variables|Configuration|GetLandmarkActivationRadius) true) ; Update radius of the landmark trigger based on Landmark\nActivation Radius (set in the Quest Map Manager component\non the player controller).
      (Components|Sphere|SetSphereRadius (Variables|Default|GetPOITrigger) (Variables|Configuration|GetPOIActivationRadius) true) ; Update radius of the POI trigger based on POI Activation\nRadius (set in the Quest Map Manager component on the\nplayer controller).
      (Components|Sphere|SetSphereRadius (Variables|Default|GetHiddenObjectTrigger) (Variables|Configuration|GetHiddenObjectActivationRadius) true) ; Update radius of the hidden object trigger based on Hidden\nObject Activation Radius (set in the Quest Map Manager\ncomponent on the player controller).
      (Components|Sphere|SetSphereRadius (Variables|Default|GetNPCTrigger) (Variables|Configuration|GetNPCActivationRadius) true) ; Update radius of the NPC trigger based on NPC Activation\nRadius (set in the Quest Map Manager component on the\nplayer controller).
      (Components|Capsule|SetCapsuleSize (Variables|Default|GetCapsuleTrigger) (.x _capsuleradius) (.y _capsuleradius) true) ; Set QuestAreaTrigget capture size based on CapsuleRadius\n(set in the Quest Map Manager component on the\nplayer controller.
      (Development|SetHiddeninGame (Variables|Default|GetNPCTrigger) (not (Variables|Configuration|GetShowOverlapVolumes)) false) ; Sets all overlap volumes to hidden or visible based on the\ndebug state bool Show Overlap Volumes (set in the Quest\nMap Manager component on the player controller).
      (Components|Sphere|SetSphereRadius (Variables|Default|GetDiscoverTrigger) (Variables|Configuration|GetDiscoverRadius) false) ; Update radius of the discovery trigger based on Discover Radius\n(set in the Quest Map Manager component on the player\ncontroller).
      (Variables|Configuration|SetInitialized true))))

(fn UpdateDiscoveryTrigger
  (Components|Sphere|SetSphereRadius (Variables|Default|GetDiscoverTrigger) (Variables|Configuration|GetDiscoverRadius) true) ; Update radius of the discovery trigger based on Discover Radius\n(set in the Quest Map Manager component on the player\ncontroller).
  (return))