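; Editor helper actor for QuestMap Pro that renders the world between NorthWest and SouthEast markers into static map textures.
; UpdateHelperActor centers it between the markers and sizes the orthographic scene capture to the world.
; CaptureMapImage saves one image, creating a render target with a power-of-two shorter side for non-square worlds.
; CaptureTieredMapImages steps the capture across each zoom tier's grid from GetCaptureSegments, optionally filling TieredZoomData with the saved segment textures.
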(fn ConstructionScript
  (bind _northwest (Variables|Configuration|GetNorthWest))
  (bind _southeast (Variables|Configuration|GetSouthEast))
  (bind _returnvalue (Transformation|GetActorLocation _southeast))
  (bind _returnvalue_2 (Transformation|GetActorLocation _northwest))
  (bind _returnvalue_3 (+ _returnvalue_2 _returnvalue))
  (bind _returnvalue_4 (/ _returnvalue_3 2.0))
  (Utilities|FlowControl|Sequence
    (:then_0
      (Variables|MapCapture|SetWarning "!!!NOTICE!!! 
 
When using \"Capture Tiered Map Images\"... 
 
This task may cause the engine to appear frozen depending on the hardware and settings used. Please give it time to complete. Task has not run this time but will run on the next attempt."))
    (:then_1
      (if (Variables|OperatingValues|GetUpdated)
        (Variables|Configuration|GetNorthWest
          (:then
            (Variables|Configuration|GetSouthEast
              (:then
                (Transformation|SetActorLocation (Math|Vector|MakeVector (.x _returnvalue_4) (.y _returnvalue_4) (.z (Transformation|GetActorLocation))) false true) ; Move helper actor to world center, maintaining current height (z axis value).
              )
              (:else
                (Variables|OperatingValues|SetUpdated false))))
          (:else
            (Variables|OperatingValues|SetUpdated false)))))))

(fn GetWorldX
  (return (Math|Float|Absolute(Float) (- (.x (Transformation|GetActorLocation (Variables|Configuration|GetNorthWest))) (.x (Transformation|GetActorLocation (Variables|Configuration|GetSouthEast)))))))

(fn GetWorldY
  (return (Math|Float|Absolute(Float) (- (.y (Transformation|GetActorLocation (Variables|Configuration|GetNorthWest))) (.y (Transformation|GetActorLocation (Variables|Configuration|GetSouthEast)))))))

(fn UpdateHelperActor
  (bind _northwest (Variables|Configuration|GetNorthWest))
  (bind _southeast (Variables|Configuration|GetSouthEast))
  (bind _returnvalue (Transformation|GetActorLocation _southeast))
  (bind _returnvalue_2 (Transformation|GetActorLocation _northwest))
  (bind _returnvalue_3 (+ _returnvalue_2 _returnvalue))
  (bind _returnvalue_4 (/ _returnvalue_3 2.0))
  (Variables|Configuration|SetWorldSize (Math|Vector2D|MakeVector2D (Configuration|GetWorldX) (Configuration|GetWorldY))) ; Calculate and save world size.
  (Transformation|SetActorLocation (Math|Vector|MakeVector (.x _returnvalue_4) (.y _returnvalue_4) (.z (Transformation|GetActorLocation))) false true) ; Move helper actor to world center, maintaining current height (z axis value).
  (Variables|/Script/Engine.SceneCaptureComponent2D|SetOrthoWidth (Variables|Default|GetMapCapture) (Math|Float|Max(Float) (.x (Variables|Configuration|GetWorldSize)) (.y (Variables|Configuration|GetWorldSize)))) ; Set map capture ortho width based on world size.
  (Variables|OperatingValues|SetUpdated true)
  (return))

(fn CaptureMapImage
  (bind _rendertargetresolution (Variables|MapCapture|GetRenderTargetResolution))
  (bind _captureheightoffset (Variables|MapCapture|GetCaptureHeightOffset))
  (bind _worldsize (Variables|Configuration|GetWorldSize))
  (bind _worldsize_2 (Variables|Configuration|GetWorldSize))
  (bind _worldsize_3 (Variables|Configuration|GetWorldSize))
  (bind _worldsize_4 (Variables|Configuration|GetWorldSize))
  (bind _returnvalue (Math|Vector|MakeVector 0.0 0.0 _captureheightoffset))
  (bind _returnvalue_2 (/ (.y _worldsize_3) (.x _worldsize_3)))
  (bind _returnvalue_3 (/ (.x _worldsize_3) (.y _worldsize_3)))
  (bind _returnvalue_4 (>= (.x _worldsize_4) (.y _worldsize_4)))
  (bind _returnvalue_5 (Utilities|Select :Index _rendertargetresolution :NewEnumerator0 512.0 :NewEnumerator1 1024.0 :NewEnumerator2 2048.0 :NewEnumerator3 4096.0 :NewEnumerator6 8192.0))
  (bind _returnvalue_6 (Math|Float|SelectFloat _returnvalue_2 _returnvalue_3 _returnvalue_4))
  (bind _returnvalue_7 (* _returnvalue_6 _returnvalue_5))
  (bind _returnvalue_8 (Math|Vector2D|MakeVector2D _returnvalue_5 _returnvalue_7))
  (bind _returnvalue_9 (Math|Vector2D|MakeVector2D _returnvalue_7 _returnvalue_5))
  (bind _returnvalue_10 (select _returnvalue_4 _returnvalue_8 _returnvalue_9))
  (bind (_x _y) (Math|Vector2D|BreakVector2D _returnvalue_10))
  (bind (_x_2 _y_2) (Math|Vector2D|BreakVector2D _returnvalue_10))
  (bind _returnvalue_11 (Math|Float|Log _y 2.0))
  (bind _returnvalue_12 (Math|Float|Log _x 2.0))
  (bind _returnvalue_13 (> _x_2 _y_2))
  (bind _returnvalue_14 (Math|Float|Ceil _returnvalue_11))
  (bind _returnvalue_15 (Math|Float|Ceil _returnvalue_12))
  (bind _returnvalue_16 (Math|Conversions|ToFloat(Integer) _returnvalue_14))
  (bind _returnvalue_17 (Math|Conversions|ToFloat(Integer) _returnvalue_15))
  (bind _returnvalue_18 (Math|Float|Power 2.0 _returnvalue_16))
  (bind _returnvalue_19 (Math|Float|Power 2.0 _returnvalue_17))
  (bind _returnvalue_20 (Math|Vector2D|MakeVector2D _returnvalue_19 _y))
  (bind _returnvalue_21 (Math|Vector2D|MakeVector2D _x _returnvalue_18))
  (bind _returnvalue_22 (select _returnvalue_13 _returnvalue_21 _returnvalue_20))
  (bind (_x_3 _y_3) (Math|Vector2D|BreakVector2D _returnvalue_22))
  (LocalVariables|SetBaseLocation (Transformation|GetActorLocation)) ; Store actor location temporarily.
  (Transformation|SetActorLocation (Math|Vector|SelectVector _returnvalue (+ _returnvalue (LocalVariables|GetBaseLocation)) (Variables|MapCapture|GetHeightOffsetIsAbsolute)) false true) ; Set the actor location to the height defined\nby Capture Height Offset, taking into\naccount whether the offset is absolute or not.
  (Variables|/Script/Engine.SceneCaptureComponent2D|SetOrthoWidth (Variables|Default|GetMapCapture) (Math|Float|Max(Float) (.x _worldsize_2) (.y _worldsize_2))) ; Set map capture ortho width based on world size.
  (if (== (.x _worldsize) (.y _worldsize))
    (Variables|/Script/Engine.SceneCaptureComponent2D|SetTextureTarget (Variables|Default|GetMapCapture) (Utilities|Select :Index (Variables|MapCapture|GetRenderTargetResolution) :NewEnumerator0 "/Game/QuestMap/MapRender/RT_QuestMapPro_WorldMapHelper_512x.RT_QuestMapPro_WorldMapHelper_512x" :NewEnumerator1 "/Game/QuestMap/MapRender/RT_QuestMapPro_WorldMapHelper_1024x.RT_QuestMapPro_WorldMapHelper_1024x" :NewEnumerator2 "/Game/QuestMap/MapRender/RT_QuestMapPro_WorldMapHelper_2048x.RT_QuestMapPro_WorldMapHelper_2048x" :NewEnumerator3 "/Game/QuestMap/MapRender/RT_QuestMapPro_WorldMapHelper_4096x.RT_QuestMapPro_WorldMapHelper_4096x" :NewEnumerator6 "/Game/QuestMap/MapRender/RT_QuestMapPro_WorldMapHelper_8192x.RT_QuestMapPro_WorldMapHelper_8192x")) ; Update the capture resolution using the\nappropriate render target texture.
    (else
      (bind _returnvalue_23 (Rendering|CreateRenderTarget2D (Math|Float|Truncate _x_3) (Math|Float|Truncate _y_3) "RTF_RGBA8"))
      (Rendering|ClearRenderTarget2D _returnvalue_23)
      (Variables|/Script/Engine.SceneCaptureComponent2D|SetTextureTarget (Variables|Default|GetMapCapture) _returnvalue_23) ; Update the capture resolution using the\nappropriate render target texture.
    ))
  (Rendering|SceneCapture|CaptureScene (Variables|Default|GetMapCapture) :!class /Script/Engine.SceneCaptureComponent2D) ; Update render target with current scene capture.
  (Class|KismetRenderingLibrary|RenderTargetCreateStaticTexture2DEditorOnly (Variables|/Script/Engine.SceneCaptureComponent2D|GetTextureTarget (Variables|Default|GetMapCapture)) (Utilities|String|Append (Variables|MapCapture|GetCaptureLocation) (Variables|MapCapture|GetCaptureName)) "TC_Default" "TMGS_FromTextureGroup") ; Create static texture of scene capture using CaptureLocation and\nCaptureName to define location and name of the texture.
  (Variables|/Script/Engine.SceneCaptureComponent2D|SetTextureTarget (Variables|Default|GetMapCapture) "/Game/QuestMap/MapRender/RT_QuestMapPro_WorldMapHelper_512x.RT_QuestMapPro_WorldMapHelper_512x") ; Set capture texture back to 512x version\njust to avoid any performance issues in the\neditor. Should not be needed but its a good\nsafety measure in case the user changes\nthe capture rates in the render texture.
  (Transformation|SetActorLocation (LocalVariables|GetBaseLocation) false true) ; Move helper actor back to base location.
  (return))

(fn CaptureTieredMapImages
  (bind _worldsize (Variables|Configuration|GetWorldSize))
  (bind _mapcapture (Variables|Default|GetMapCapture))
  (if (Variables|MapCapture|GetEnableTieredZoomTransitions) ; Only execute this function if tiered zoom transitions are enabled.
    (LocalVariables|SetActorBaseLocation (Transformation|GetActorLocation)) ; Cache current actor location (used for resetting after function completion)
    (if (Variables|MapCapture|GetAutomaticallyPopulateTexturesForMap) ; Should capture data be stored for automatic population of\nTiered Zoom Data?
      (Utilities|Array|Clear (Variables|MapCapture|GetTieredZoomData)) ; Clear current TieredZoomData.
    )
    (for (_array_element _array_index) (Variables|MapCapture|GetTieredZoomTransitions) ; For each tiered zoom transition defined...
      (LocalVariables|SetElementData _array_element) ; Cache element data.
      (LocalVariables|SetIndex _array_index) ; Cache element index.
      (if (Variables|MapCapture|GetAutomaticallyPopulateTexturesForMap) ; Should capture data be stored for automatic population of\nTiered Zoom Data?
        (Utilities|Array|Add (Variables|MapCapture|GetTieredZoomData) (Utilities|Struct|MakeStr_QuestMapPro_ZoomTierReferenceData (.TransitionZoom (Utilities|Struct|BreakStr_QuestMapPro_ZoomTierData (LocalVariables|GetElementData))) (.GridDimensions (Utilities|Struct|BreakStr_QuestMapPro_ZoomTierData (LocalVariables|GetElementData))))) ; Add new entry into TieredZoomData,\npopulating TransitionZoom and Grid\nDimensions from current element.
      )
      (bind _capturelocations (MapCapture|GetCaptureSegments (LocalVariables|GetIndex))) ; Get an array of locations that will be used for captures.
      (LocalVariables|SetLocations _capturelocations) ; Cache capture locations.
      (Variables|/Script/Engine.SceneCaptureComponent2D|SetOrthoWidth (Variables|Default|GetMapCapture) (/ (Math|Float|Max(Float) (.x _worldsize) (.y _worldsize)) (Math|Conversions|ToFloat(Integer) (.GridDimensions (Utilities|Struct|BreakStr_QuestMapPro_ZoomTierData (LocalVariables|GetElementData)))))) ; Set map capture ortho width based on world size.
      (Variables|/Script/Engine.SceneCaptureComponent2D|SetTextureTarget (Variables|Default|GetMapCapture) (Utilities|Select :Index (.SegmentResolution (Utilities|Struct|BreakStr_QuestMapPro_ZoomTierData (LocalVariables|GetElementData))) :NewEnumerator0 "/Game/QuestMap/MapRender/RT_QuestMapPro_WorldMapHelper_512x.RT_QuestMapPro_WorldMapHelper_512x" :NewEnumerator1 "/Game/QuestMap/MapRender/RT_QuestMapPro_WorldMapHelper_1024x.RT_QuestMapPro_WorldMapHelper_1024x" :NewEnumerator2 "/Game/QuestMap/MapRender/RT_QuestMapPro_WorldMapHelper_2048x.RT_QuestMapPro_WorldMapHelper_2048x" :NewEnumerator3 "/Game/QuestMap/MapRender/RT_QuestMapPro_WorldMapHelper_4096x.RT_QuestMapPro_WorldMapHelper_4096x" :NewEnumerator6 "/Game/QuestMap/MapRender/RT_QuestMapPro_WorldMapHelper_8192x.RT_QuestMapPro_WorldMapHelper_8192x")) ; Set render target texture based on\nsegment resolution defined in current\nelement data.
      (for (_array_element_2 _array_index_2) (LocalVariables|GetLocations) ; For each capture location...
        (Transformation|SetActorLocation _array_element_2 false true) ; Move helper to location.
        (Rendering|SceneCapture|CaptureScene _mapcapture :!class /Script/Engine.SceneCaptureComponent2D) ; Capture scene at location.
        (bind _returnvalue (Class|KismetRenderingLibrary|RenderTargetCreateStaticTexture2DEditorOnly (Variables|/Script/Engine.SceneCaptureComponent2D|GetTextureTarget _mapcapture) (Utilities|String|Append (Variables|MapCapture|GetCaptureLocation) (Utilities|String|Append "Zoom" (Utilities|String|ToString(Integer) (LocalVariables|GetIndex))) "/" (Variables|MapCapture|GetCaptureName) "_" (Utilities|String|Append "Zoom" (Utilities|String|ToString(Integer) (LocalVariables|GetIndex))) "_" (Utilities|String|ToString(Integer) _array_index_2)) "TC_Default" "TMGS_FromTextureGroup")) ; Render captured scene out as a texture.
        (if (Variables|MapCapture|GetAutomaticallyPopulateTexturesForMap) ; Should capture data be stored for automatic population of\nTiered Zoom Data?
          (Utilities|Array|Add (Utilities|Struct|BreakStr_QuestMapPro_ZoomTierReferenceData (Utilities|Array|Get(acopy) (Variables|MapCapture|GetTieredZoomData) (LocalVariables|GetIndex))) _returnvalue) ; Add capture to SegmentTextures array at current element.
        )))
    (Transformation|SetActorLocation (LocalVariables|GetActorBaseLocation) false true) ; Move helper actor back to base location.
    (return)
    (else
      (Development|PrintString "Tiered Zoom Transitions are not enabled. Use CaptureMapImage to capture map if only a single image is required.") ; Notify user of reason capture did not execute.
      (return))))

(fn GetCaptureSegments
  (params (TierIndex :type Integer))
  (bind _captureheightoffset (Variables|MapCapture|GetCaptureHeightOffset))
  (bind _northwest (Variables|Configuration|GetNorthWest))
  (bind _tieredzoomtransitions (Variables|MapCapture|GetTieredZoomTransitions))
  (bind _returnvalue (Transformation|GetActorLocation _northwest))
  (bind _returnvalue_2 (Math|Vector|MakeVector 0.0 0.0 _captureheightoffset))
  (bind _output (Utilities|Array|Get(acopy) _tieredzoomtransitions TierIndex))
  (bind _griddimensions (Utilities|Struct|BreakStr_QuestMapPro_ZoomTierData _output))
  (bind _returnvalue_3 (Math|Conversions|ToFloat(Integer) _griddimensions))
  (Utilities|Array|Clear (LocalVariables|GetLocations)) ; Clear locations array.\nRedundancy measure.\nShould never be needed.
  (LocalVariables|SetXOffset 0.0) ; Set initial XOffset to 0.\nRedundancy measure.\nShould never be needed.
  (LocalVariables|SetYOffset 0.0) ; Set initial YOffset to 0.\nRedundancy measure.\nShould never be needed.
  (LocalVariables|SetX (/ (Configuration|GetWorldX) (* _returnvalue_3 2.0))) ; Calculate value that represents half\ndistance along X axis between\nsegments.
  (LocalVariables|SetY (/ (Configuration|GetWorldY) (* _returnvalue_3 2.0))) ; Calculate value that represents half\ndistance along Y axis between\nsegments.
  (for _index (range 0 (- (* _griddimensions _griddimensions) 1)) ; For every single grid segment...\n(GridDimensions squared - 1 to account for 0 index)
    (LocalVariables|SetLoopX (+ (Math|Integer|%(Integer) _index (Math|Float|Truncate _returnvalue_3)) 1)) ; Calculate X value (column) using modulus.
    (LocalVariables|SetLoopY (+ (/ _index (Math|Float|Truncate _returnvalue_3)) 1)) ; Calculate Y value (row) by using integer results of division.
    (LocalVariables|SetXOffset (+ (Math|Float|SelectFloat 0.0 (LocalVariables|GetXOffset) (== (LocalVariables|GetLoopX) 1)) (* (LocalVariables|GetX) (Math|Float|SelectFloat 1.0 2.0 (== (LocalVariables|GetLoopX) 1))))) ; Calculate X offset for this segment.
    (LocalVariables|SetYOffset (- (* (LocalVariables|GetY) (* (Math|Conversions|ToFloat(Integer) (LocalVariables|GetLoopY)) (Math|Float|SelectFloat 1.0 2.0 (== (LocalVariables|GetLoopY) 1)))) (Math|Float|SelectFloat 0.0 (LocalVariables|GetY) (== (LocalVariables|GetLoopY) 1)))) ; Calculate Y offset for this segment.
    (Utilities|Array|Add (LocalVariables|GetLocations) (Math|Vector|MakeVector (+ (LocalVariables|GetXOffset) (.x _returnvalue)) (+ (.y _returnvalue) (LocalVariables|GetYOffset)) (.z (Math|Vector|SelectVector _returnvalue_2 (+ _returnvalue_2 (Transformation|GetActorLocation)) (Variables|MapCapture|GetHeightOffsetIsAbsolute))))) ; Add location to Locations array.
  )
  (return (LocalVariables|GetLocations)))