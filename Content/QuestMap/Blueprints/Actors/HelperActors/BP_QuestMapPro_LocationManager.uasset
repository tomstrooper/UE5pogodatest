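; BP_QuestMapPro_LocationManager is a Quest Map Pro helper actor that maintains the array of known landmarks, each pairing a landmark actor with a state.
; CollectAllLandmarks rebuilds the array from every landmark actor in the scene using the default state, first saving a backup independent of the undo buffer.
; RetrieveCustomList restores that backup.
; SetAllKnownLandmarksState resets every entry to the default state.
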(fn ConstructionScript)

(fn CollectAllLandmarks
  (Variables|Landmarks|SetCustomLandmarks (Variables|Landmarks|GetKnownLandmarks)) ; Backup custom list of landmarks for\nundo irrespective of undo buffer.
  (Utilities|Array|Clear (Variables|Landmarks|GetKnownLandmarks)) ; Clear known landmarks.
  (bind _outactors (Actor|GetAllActorsOfClass "/Game/QuestMap/Blueprints/Actors/WorldObjects/BP_QuestMapPro_Landmark.BP_QuestMapPro_Landmark_C")) ; Get all landmark actors in the scene.
  (for _array_element _outactors ; For each landmark actor in the scene...
    (Utilities|Array|Add (Variables|Landmarks|GetKnownLandmarks) (Utilities|Struct|MakeStr_QuestMapPro_LandmarkData _array_element (Variables|Landmarks|GetDefaultLandmarkState))) ; Add landmark to known landmark array.
  )
  (return))

(fn RetrieveCustomList
  (Utilities|Array|Clear (Variables|Landmarks|GetKnownLandmarks)) ; Clear known landmarks.
  (Variables|Landmarks|SetKnownLandmarks (Variables|Landmarks|GetCustomLandmarks)) ; Set known landmarks to custom landmarks backup.
  (return))

(fn SetAllKnownLandmarksState
  (for (_array_element _array_index) (Variables|Landmarks|GetKnownLandmarks) ; For every unknown landmark...
    (bind _structout (Utilities|Struct|SetmembersinStr_QuestMapPro_LandmarkData _array_element (Variables|Landmarks|GetDefaultLandmarkState))) ; Update landmark state with default state.
    (Utilities|Array|SetArrayElem (Variables|Landmarks|GetKnownLandmarks) _array_index _structout) ; Update entry in array with new struct.
  )
  (return))