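; Quest map navigation helper actor that stores route points as splines and animates a Niagara trail effect along the path.
; SetNavPath builds a linear spline, while SetTrailPath builds a curved one, clamping tangents at closely spaced points, then starts the effect.
; A speed-scaled timeline moves the effect by spline distance and triggers particle spawn and kill.
; Line traces keep it just above the ground, and it hides when progress stalls or ends.
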(event Custom|StartEffect
  (if (not (Variables|Default|GetEffectInProgress)) ; Is the effect currently active?
    (CallFunction|SetEffectVisibility true) ; Set effect visibility to on.
    (Variables|Default|SetEffectInProgress true) ; Update current effect state.
    (bind _alpha (Timeline|SplineLerpAlpha PlayFromStart)
      (:Update
        (Variables|Default|SetUpdateAlpha (* (Math|Float|Clamp(Float) _alpha 0.0 (/ (Spline|GetSplineLength (Variables|Default|GetTrailPath)) (Variables|Default|GetTrailPathDistance))) (Variables|Default|GetTrailPathDistance))) ; Use timeline alpha to find current alpha along the spline.
        (if (Math|Float|NearlyEqual(Float) (Variables|Default|GetUpdateAlpha) (Variables|Default|GetPriorAlpha) 1e-06) ; Is the update alpha nearly the same as\nthe prior alpha?
          (CallFunction|SetEffectVisibility false) ; Set effect visibility to off.
          (else
            (Variables|Default|SetPriorAlpha (Variables|Default|GetUpdateAlpha)) ; Update PrioAlpha with new alpha.
            (Transformation|SetWorldLocationAndRotation (Variables|Default|GetEffect) (Math|Vector|MakeVector (.X (Math|Vector|BreakVector (.Location (Math|Transform|BreakTransform (Spline|GetTransformatDistanceAlongSpline (Variables|Default|GetTrailPath) (Variables|Default|GetUpdateAlpha) "World" false))))) (.Y (Math|Vector|BreakVector (.Location (Math|Transform|BreakTransform (Spline|GetTransformatDistanceAlongSpline (Variables|Default|GetTrailPath) (Variables|Default|GetUpdateAlpha) "World" false))))) (CallFunction|GetEffectHeight (.Location (Math|Transform|BreakTransform (Spline|GetTransformatDistanceAlongSpline (Variables|Default|GetTrailPath) (Variables|Default|GetUpdateAlpha) "World" false))))) (.Rotation (Math|Transform|BreakTransform (Spline|GetTransformatDistanceAlongSpline (Variables|Default|GetTrailPath) (Variables|Default|GetUpdateAlpha) "World" false))) false true) ; Move effect to appropriate location along spline.
            (CallFunction|SetEffectVisibility true) ; Set effect visibility to on.
          )))
      (:Finished
        (Variables|Default|SetEffectInProgress false) ; Update effect state.
        (CallFunction|SetEffectVisibility false) ; Hide the effect.
        (Utilities|IsValid (Variables|Default|GetActiveParticle) ; Avoid trying to kill the particle if it has\nalready been killed.
          (:Is%20Valid
            (Components|DestroyComponent (Variables|Default|GetActiveParticle)) ; Kill the particle.
          )))
      (:SpawnParticle
        (bind _returnvalue (Niagara|SpawnSystemAttached (AssetData|GetAsset (Variables|Default|GetNiagara)) (Variables|Default|GetEffect) "None" "0, 0, 0" "0, 0, 0" "KeepRelativeOffset" false)) ; Spawn new instance of particle effect.
        (Variables|Default|SetActiveParticle _returnvalue) ; Store reference to effect for killing later.
      )
      (:KillParticle
        (Components|DestroyComponent (Variables|Default|GetActiveParticle)) ; Kil the particle.
      ))))

(event Custom|StopEffect
  (Utilities|FlowControl|Sequence ; Execute in order:\n1: Stop timeline\n2: Update effect state/visibility
    (:then_0
      (bind _alpha (Timeline|SplineLerpAlpha Stop)
        (:Update
          (Variables|Default|SetUpdateAlpha (* (Math|Float|Clamp(Float) _alpha 0.0 (/ (Spline|GetSplineLength (Variables|Default|GetTrailPath)) (Variables|Default|GetTrailPathDistance))) (Variables|Default|GetTrailPathDistance))) ; Use timeline alpha to find current alpha along the spline.
          (if (Math|Float|NearlyEqual(Float) (Variables|Default|GetUpdateAlpha) (Variables|Default|GetPriorAlpha) 1e-06) ; Is the update alpha nearly the same as\nthe prior alpha?
            (CallFunction|SetEffectVisibility false) ; Set effect visibility to off.
            (else
              (Variables|Default|SetPriorAlpha (Variables|Default|GetUpdateAlpha)) ; Update PrioAlpha with new alpha.
              (Transformation|SetWorldLocationAndRotation (Variables|Default|GetEffect) (Math|Vector|MakeVector (.X (Math|Vector|BreakVector (.Location (Math|Transform|BreakTransform (Spline|GetTransformatDistanceAlongSpline (Variables|Default|GetTrailPath) (Variables|Default|GetUpdateAlpha) "World" false))))) (.Y (Math|Vector|BreakVector (.Location (Math|Transform|BreakTransform (Spline|GetTransformatDistanceAlongSpline (Variables|Default|GetTrailPath) (Variables|Default|GetUpdateAlpha) "World" false))))) (CallFunction|GetEffectHeight (.Location (Math|Transform|BreakTransform (Spline|GetTransformatDistanceAlongSpline (Variables|Default|GetTrailPath) (Variables|Default|GetUpdateAlpha) "World" false))))) (.Rotation (Math|Transform|BreakTransform (Spline|GetTransformatDistanceAlongSpline (Variables|Default|GetTrailPath) (Variables|Default|GetUpdateAlpha) "World" false))) false true) ; Move effect to appropriate location along spline.
              (CallFunction|SetEffectVisibility true) ; Set effect visibility to on.
            )))
        (:Finished
          (Variables|Default|SetEffectInProgress false :!label _label) ; Update effect state.
          (CallFunction|SetEffectVisibility false) ; Hide the effect.
          (Utilities|IsValid (Variables|Default|GetActiveParticle) ; Avoid trying to kill the particle if it has\nalready been killed.
            (:Is%20Valid
              (Components|DestroyComponent (Variables|Default|GetActiveParticle)) ; Kill the particle.
            )))
        (:SpawnParticle
          (bind _returnvalue (Niagara|SpawnSystemAttached (AssetData|GetAsset (Variables|Default|GetNiagara)) (Variables|Default|GetEffect) "None" "0, 0, 0" "0, 0, 0" "KeepRelativeOffset" false)) ; Spawn new instance of particle effect.
          (Variables|Default|SetActiveParticle _returnvalue) ; Store reference to effect for killing later.
        )
        (:KillParticle
          (Components|DestroyComponent (Variables|Default|GetActiveParticle)) ; Kil the particle.
        )))
    (:then_1
      (goto _label))))

(event EventBeginPlay
  (Components|Timeline|SetPlayRate (Variables|Default|GetSplineLerpAlpha) (Variables|Default|GetTrailPathSpeed)) ; Set effect path speed based on\nTrailPathSpeed (set on spawn).
  (Variables|Default|SetEffectInProgress false) ; Clear current effect state.
  (CallFunction|SetEffectVisibility false) ; Set initial effect visibility to off.
)

(fn ConstructionScript)

(fn SetNavPath
  (params (PathPoints :type Array%20of%20Vectors))
  (LocalVariables|SetPath PathPoints) ; Cache input.
  (Spline|ClearSplinePoints (Variables|Default|GetNavPath) true) ; Clear current nav path spline.
  (for (_array_element _array_index) (LocalVariables|GetPath) ; For each path vector...
    (Spline|AddSplinePoint (Variables|Default|GetNavPath) _array_element "World" false) ; Add spline point to Nav Path.
    (Spline|SetSplinePointType (Variables|Default|GetNavPath) _array_index "Linear" false) ; Set spline point type to Linear.
  )
  (Spline|UpdateSpline (Variables|Default|GetNavPath)) ; Update spline once all points added.
  (return))

(fn SetTrailPath
  (params (PathPoints :type Array%20of%20Vectors))
  (LocalVariables|SetPath PathPoints) ; Cache input.
  (Spline|ClearSplinePoints (Variables|Default|GetTrailPath) true) ; Clear current trail path spline.
  (for (_array_element _array_index) (LocalVariables|GetPath) ; For each path vector...
    (Spline|AddSplinePoint (Variables|Default|GetTrailPath) _array_element "World" false) ; Add spline point to Trail Path.
    (Spline|SetSplinePointType (Variables|Default|GetTrailPath) _array_index (select (or (< (Math|Vector|Distance(Vector) _array_element (Utilities|Array|Get(acopy) (LocalVariables|GetPath) (Math|Integer|Clamp(Integer) (+ _array_index -1) 0 (Utilities|Array|LastIndex (LocalVariables|GetPath))))) 1e+03) (< (Math|Vector|Distance(Vector) _array_element (Utilities|Array|Get(acopy) (LocalVariables|GetPath) (Math|Integer|Clamp(Integer) (+ _array_index 1) 0 (Utilities|Array|LastIndex (LocalVariables|GetPath))))) 1e+03)) "CurveClamped" "Curve") false) ; Set spline point type.
  )
  (Spline|UpdateSpline (Variables|Default|GetTrailPath)) ; Update spline once all points added.
  (CallFunction|StartEffect) ; Initiate effect.
  (return))

(fn SetEffectVisibility
  (params (NewState :type Boolean))
  (if (Math|Boolean|Equal(Boolean) NewState (Variables|/Script/Engine.SceneComponent|GetbVisible (Variables|Default|GetEffect))) ; Is the input state the same as the current state?
    (return)
    (else
      (Rendering|SetVisibility (Variables|Default|GetEffect) NewState true) ; Update visibility based on input.
      (return))))

(fn GetEffectHeight
  (params (Location :type Vector))
  (bind (_outhit _returnvalue) (Collision|LineTraceByChannel (+ Location "0, 0,500.000000") (- Location "0,0.000000,500.000000") "TraceTypeQuery1" false 0 "None")) ; Do a small trace from 500 units above the current location to\n500 units below the current location (1000 units in total) to look\nfor the "ground".
  (if _returnvalue ; Was a hit made?
    (return (+ (.Z (Math|Vector|BreakVector (.Location (Collision|BreakHitResult _outhit)))) 2e+01)) ; Use height (z value) of hit location.
    (else
      (return (.z Location)) ; Use input height (z value).
    )))