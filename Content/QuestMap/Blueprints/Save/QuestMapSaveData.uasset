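; QuestMapSaveData holds the quest map's saved data: landmarks, notes, POIs and waypoints.
; It exposes one getter per collection, each returning the stored variable directly with no filtering or other logic.
; The graphs shown only read this data and contain no code that writes, saves or loads it.
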(fn GetLandmarks
  (return (Variables|Default|GetLandmarks)))

(fn GetNotes
  (return (Variables|Default|GetNotes)))

(fn GetPOIs
  (return (Variables|Default|GetPOIs)))

(fn GetWaypoints
  (return (Variables|Default|GetWaypoints)))